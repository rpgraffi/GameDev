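; BP_Deckenlicht is a ceiling light actor that can be switched on and off and registers itself with a lights manager.
; On BeginPlay it adds itself to the LightArray of its LightsManager reference, or prints a warning with its name if that reference is invalid.
; ToggleLight flips the visibility of the root component and propagates the change to its children.
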(event EventBeginPlay
  (bind _lightsmanager (Variables|Default|GetLightsManager)
    (:then
      (Utilities|Array|Add (Variables|/Game/Dynamic/Environment/Lights/BP_LightsManager.BP_LightsManager_C|GetLightArray _lightsmanager) self))
    (:else
      (Development|PrintString (Utilities|String|Append (Utilities|String|ToString(Object) self) (Utilities|String|MakeLiteralString " not connected to Light Manager"))))))

(fn ConstructionScript)

(fn ToggleLight
  (Rendering|ToggleVisibility (Variables|Default|GetDefaultSceneRoot) true))