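; BP_LightsManager is a manager that controls a group of BP_Deckenlicht ceiling lights as one unit.
; On BeginPlay it loops over LightArray and sets the lights on or off according to IsOn, stopping at any entry that fails the cast.
; The Hebeln event calls ToggleLights, which flips each light individually without updating IsOn and prints a warning for invalid entries.
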(event EventBeginPlay
  (for _array_element (Variables|Default|GetLightArray)
    (bind _asbp_deckenlicht (Utilities|Casting|CastToBP_Deckenlicht _array_element))
    (if (Variables|Default|GetisOn)
      (Default|Lighton _asbp_deckenlicht)
      (else
        (Default|LightOff _asbp_deckenlicht)))))

(event EventHebeln
  (CallFunction|ToggleLights))

(fn ConstructionScript)

(fn ToggleLights
  (for _array_element (Variables|Default|GetLightArray)
    (bind _asbp_deckenlicht (Utilities|Casting|CastToBP_Deckenlicht _array_element)
      (:then
        (Default|ToggleLight _asbp_deckenlicht))
      (:CastFailed
        (Development|PrintString "Invalid Light in BP_LightManager")))))