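; BP_KeyPad_Button is a single clickable button for an in-game keypad, labeled from its NumberText variable in the construction script.
; Cursor-over events swap the button's material to show hover, and ResetButtons restores the default material.
; On release it plays a click sound and calls ButtonClicked on its KeypadReference, passing the text plus confirm and backspace flags.
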(event OnBeginCursorOver(Button)
  (params (TouchedComponent :type Primitive%20Component%20Object%20Reference))
  ;[1 1 1] Hover / Unhover effects
  (Rendering|Material|SetMaterial (Variables|Default|GetButton) 0 "/Game/Dynamic/Environment/Keypad/Materials/MI_KeyPad_ButtonTouched.MI_KeyPad_ButtonTouched") ; Material to switch to when hovered
)

(event OnEndCursorOver(Button)
  (params (TouchedComponent :type Primitive%20Component%20Object%20Reference))
  ;[1 1 1] Hover / Unhover effects
  (Rendering|Material|SetMaterial (Variables|Default|GetButton) 0 "/Game/Dynamic/Environment/Keypad/Materials/MI_KeyPad_Button.MI_KeyPad_Button"))

(event OnReleased(Button)
  (params (TouchedComponent :type Primitive%20Component%20Object%20Reference) (ButtonReleased :type Key%20Structure :default "None"))
  ;[1 1 1] On Button Click Event
  (Audio|PlaySound2D "/Game/Static/SoundEffects/WAV/Click_06.Click_06" 1.0 1.0 0.0 0 0)
  (Default|ButtonClicked (Variables|Default|GetKeypadReference) (Variables|Default|GetNumberText) (Variables|Default|GetConfirmedButton?) (Variables|Default|GetBackspaceButton?)))

(event Custom|ResetButtons
  ;[1 1 1] Hover / Unhover effects
  (Rendering|Material|SetMaterial (Variables|Default|GetButton) 0 "/Game/Dynamic/Environment/Keypad/Materials/MI_KeyPad_Button.MI_KeyPad_Button"))

(fn ConstructionScript
  ;[1 1 1] Set initial Text
  (Rendering|Components|TextRender|SetText (Variables|Default|GetButtonNumber) (Variables|Default|GetNumberText)))