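; BP_SoundActor is a trigger-zone actor that plays a 2D sound, apparently a voice line, when an actor implementing BPI_SoundActor overlaps it.
; It uses the player's CurrentSoundPlayingActor to coordinate playback, cutting off the current sound if skippable, otherwise playing only if that one has finished.
; Timers set to the sound's duration reset the playing flag and destroy the actor when it cannot be replayed.
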(event OnComponentBeginOverlap(TriggerZone)
  (params (OverlappedComponent :type Primitive%20Component%20Object%20Reference) (OtherActor :type Actor%20Object%20Reference) (OtherComp :type Primitive%20Component%20Object%20Reference) (OtherBodyIndex :type Integer) (bFromSweep :type Boolean) (SweepResult :type Hit%20Result%20Structure%20%28by%20ref%29))
  (if (Utilities|DoesObjectImplementInterface OtherActor "/Game/Dynamic/FirstPerson/Blueprints/BPI_SoundActor.BPI_SoundActor_C")
    (bind _currentsoundplayingactor (Variables|/Game/Dynamic/Core/BP_Character.BP_Character_C|GetCurrentSoundPlayingActor (Variables|Default|GetBPCharacter))
      (:then
        (if (== _currentsoundplayingactor self)
          (if (not (Variables|Default|GetisPlayingSound))
            (bind _returnvalue (Audio|SpawnSound2D (Variables|Default|GetSound) 1.0 1.0 0.0 0 :!label _label))
            (Variables|Default|SetAudioComponent _returnvalue)
            (Variables|Default|SetisPlayingSound true)
            (Utilities|Time|SetTimerbyFunctionName 0 "ResetCanPlaySound" (Variables|Default|GetDuration))
            (if (not (Variables|Default|GetcanBePlayedAgain))
              (Utilities|Time|SetTimerbyFunctionName 0 "DestroyVoiceActor" (Variables|Default|GetDuration))))
          (elif (Variables|BP_SoundActor_C|GetisSkippable _currentsoundplayingactor)
            (CallFunction|StopSound _currentsoundplayingactor)
            (if (Variables|BP_SoundActor_C|GetcanBePlayedAgain _currentsoundplayingactor)
              _
              (else
                (CallFunction|DestroyVoiceActor _currentsoundplayingactor)))
            (Variables|/Game/Dynamic/Core/BP_Character.BP_Character_C|SetCurrentSoundPlayingActor (Variables|Default|GetBPCharacter) self :!label _label_2)
            (goto _label)
            (elif (not (Variables|BP_SoundActor_C|GetisPlayingSound _currentsoundplayingactor))
              (goto _label_2)))))
      (:else
        (goto _label_2)))))

(event EventBeginPlay
  (Variables|Default|SetDuration (Variables|/Script/Engine.SoundBase|GetDuration (Variables|Default|GetSound)))
  (bind _asbp_character (Utilities|Casting|CastToBP_Character (Game|GetPlayerCharacter 0)))
  (Variables|Default|SetBPCharacter _asbp_character))

(fn ConstructionScript)

(fn ResetCanPlaySound
  (Variables|Default|SetisPlayingSound false))

(fn StopSound
  (bind _audiocomponent (Variables|Default|GetAudioComponent)
    (:then
      (Audio|Components|Audio|Stop _audiocomponent))
    (:else)))

(fn DestroyVoiceActor
  (Components|DestroyComponent (Variables|Default|GetAudioComponent))
  (Actor|DestroyActor))