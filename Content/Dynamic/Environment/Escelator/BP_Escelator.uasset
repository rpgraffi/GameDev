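; Spline-driven escalator with looping, reversible steps, toggled on and off by the Hebeln event.
; The construction script spawns width-scaled step meshes along the spline, registering them in StepArray only when HasGlassWalls is set, alongside static side walls.
; While running, Tick advances one shared distance at constant speed, places registered steps at wrapped offsets using yaw-only rotation, and plays SWEscalator.
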(event EventTick
  (params (DeltaSeconds :type Float%20%28single-precision%29))
  (bind _spline (Variables|Default|GetSpline))
  (bind _sw_escalator (Variables|Default|GetSW_Escalator))
  (bind _spline_2 (Variables|Default|GetSpline))
  (bind _returnvalue (Spline|GetSplineLength _spline_2))
  (if (Utilities|Array|IsValidIndex (Variables|Default|GetStepArray))
    (if (Variables|Default|GetisRunning)
      (if (Audio|Components|Audio|IsPlaying _sw_escalator)
        _
        (else
          (Audio|Components|Audio|Play _sw_escalator 0.0)))
      (Variables|Default|SetDistanceAlongSpline (Math|Interpolation|FInterptoConstant (Variables|Default|GetDistanceAlongSpline) (Math|Float|SelectFloat 0.0 (Spline|GetSplineLength (Variables|Default|GetSpline)) (Variables|Default|GetisReverse)) (Utilities|Time|GetWorldDeltaSeconds) (Variables|Default|GetInterpSpeed)))
      (for (_array_element _array_index) (Variables|Default|GetStepArray)
        (Transformation|SetWorldLocationAndRotation _array_element (Spline|GetLocationatDistanceAlongSpline _spline (Math|Float|SelectFloat (- (+ (Variables|Default|GetDistanceAlongSpline) (* _array_index (Variables|Default|GetStepOffset))) _returnvalue) (+ (Variables|Default|GetDistanceAlongSpline) (* _array_index (Variables|Default|GetStepOffset))) (> (+ (Variables|Default|GetDistanceAlongSpline) (* _array_index (Variables|Default|GetStepOffset))) _returnvalue)) "World") (Math|Rotator|MakeRotator 0.0 0.0 (.yaw (Spline|GetRotationatDistanceAlongSpline _spline (Math|Float|SelectFloat (- (+ (Variables|Default|GetDistanceAlongSpline) (* _array_index (Variables|Default|GetStepOffset))) _returnvalue) (+ (Variables|Default|GetDistanceAlongSpline) (* _array_index (Variables|Default|GetStepOffset))) (> (+ (Variables|Default|GetDistanceAlongSpline) (* _array_index (Variables|Default|GetStepOffset))) _returnvalue)) "World"))) false false))
      (if (Math|Float|NearlyEqual(Float) (Variables|Default|GetDistanceAlongSpline) (Math|Float|SelectFloat 0.0 (Spline|GetSplineLength (Variables|Default|GetSpline)) (Variables|Default|GetisReverse)) 0.01)
        (Variables|Default|SetDistanceAlongSpline (Math|Float|SelectFloat (Spline|GetSplineLength (Variables|Default|GetSpline)) 0.0 (Variables|Default|GetisReverse))))
      (else
        (Audio|Components|Audio|Stop _sw_escalator)))))

(event EventHebeln
  (if (Variables|Default|GetisRunning)
    (Variables|Default|SetisRunning false)
    (else
      (Variables|Default|SetisRunning true))))

(fn ConstructionScript
  (bind _spline (Variables|Default|GetSpline))
  (bind _spline_2 (Variables|Default|GetSpline))
  (Utilities|Array|Clear (Variables|Default|GetStepArray))
  (for _index (range 0 (Math|Float|Floor (/ (Spline|GetSplineLength (Variables|Default|GetSpline)) (Variables|Default|GetStepOffset))))
    (bind _returnvalue (AddComponent|AddStaticMeshComponent false (Math|Transform|MakeTransform (Spline|GetLocationatDistanceAlongSpline _spline_2 (* _index (Variables|Default|GetStepOffset)) "Local") (Math|Rotator|MakeRotator 0.0 0.0 (.yaw (Spline|GetRotationatDistanceAlongSpline _spline_2 (* _index (Variables|Default|GetStepOffset)) "Local"))) (Math|Vector|MakeVector 1.0 (Variables|Default|GetStairWidth) 1.0))))
    (if (Variables|Default|GethasGlassWalls)
      (Utilities|Array|Add (Variables|Default|GetStepArray) _returnvalue)
      (for _index_2 (range 1 2)
        (AddComponent|AddStaticMeshComponent false (Math|Transform|MakeTransform (Math|Vector|MakeVector (.x (Spline|GetLocationatDistanceAlongSpline _spline (* _index (Variables|Default|GetStepOffset)) "Local")) (+ (.y (Spline|GetLocationatDistanceAlongSpline _spline (* _index (Variables|Default|GetStepOffset)) "Local")) (* (Variables|Default|GetStairWidth) (* (Math|Integer|SelectInt _index_2 -1 (== _index_2 1)) 75))) (+ (.z (Spline|GetLocationatDistanceAlongSpline _spline (* _index (Variables|Default|GetStepOffset)) "Local")) 2e+01)) (Math|Rotator|MakeRotator (.pitch (Spline|GetRotationatDistanceAlongSpline _spline (* _index (Variables|Default|GetStepOffset)) "Local")) 0.0 (+ (.yaw (Spline|GetRotationatDistanceAlongSpline _spline (* _index (Variables|Default|GetStepOffset)) "Local")) 9e+01)) (Math|Conversions|ToVector(Float) 1.0)))))))