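; BP_Hebel is an interactable lever that signals its target actors and clears an invisible escalator barrier.
; Interact plays a fall sound and runs a timeline forward or in reverse to rotate the pivot, based on an up/down flag that Tick derives from the timeline value.
; When the timeline finishes, it plays a break sound, calls HebelnMessage on each target and destroys the barrier if valid.
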(event EventTick
  (params (DeltaSeconds :type Float%20%28single-precision%29))
  (Variables|Default|SetisLeverUp (> (stale EventInteract _hebel) 1.0)))

(event EventInteract
  (bind _invisiblebarrierescalator (Variables|Default|GetInvisibleBarrierEscalator))
  (Audio|PlaySoundatLocation "/Game/Dynamic/Environment/Hebel/SW_Lever_Fall.SW_Lever_Fall" (Transformation|GetWorldLocation (Variables|Default|GetHebel)) "0, 0, 0" 1.0 1.0 0.0 0 0 0 0)
  (if (Variables|Default|GetisLeverUp)
    (bind _hebel (Timeline|LeverTimeline Reverse)
      (:Update
        (Transformation|SetRelativeRotation (Variables|Default|GetPivotPoint) (Math|Rotator|MakeRotator -9e+01 0.0 _hebel) false false))
      (:Finished
        (Audio|PlaySoundatLocation "/Game/Dynamic/Environment/Hebel/SW_Lever_Break.SW_Lever_Break" (Transformation|GetWorldLocation (Variables|Default|GetHebel)) "0, 0, 0" 1.0 1.0 0.0 0 0 0 0)
        (for _array_element (Variables|Default|GetTargetActor)
          (Class|BPIHebel|Hebeln(Message) _array_element)
          (if (Utilities|IsValid _invisiblebarrierescalator)
            (Actor|DestroyActor _invisiblebarrierescalator)))))
    (else
      (Timeline|LeverTimeline Play))))

(fn ConstructionScript)