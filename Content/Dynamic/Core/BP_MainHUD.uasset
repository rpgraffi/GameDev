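; Main HUD that creates the root UI_Manager widget for the owning player and serves as the entry point for layered UI.
; On BeginPlay it passes InitialScreens to the manager, stores it as PrimaryLayout and adds it to the viewport.
; Its functions are thin wrappers that forward layer registration, content push and pop, and clearing calls to that layout.
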(event EventBeginPlay
  (bind _returnvalue (UserInterface|CreateWidget "/Game/Dynamic/UI/Layout/UI_Manager.UI_Manager_C" (Game|Player|GetOwningPlayerController) (Variables|Config|GetInitialScreens)))
  (bind _output_get (Variables|State|SetPrimaryLayout _returnvalue))
  (UserInterface|Viewport|AddtoViewport _output_get 0)
  (Development|PrintString "Added UI Manager"))

(fn ConstructionScript)

(fn GetPrimaryLayout
  (return (Variables|State|GetPrimaryLayout)))

(fn RegisterLayer
  (params (LayerName :type Gameplay%20Tag%20Structure) (LayerWidget :type WBP%20Layer%20Object%20Reference))
  (bind _returnvalue (Default|RegisterLayer (CallFunction|GetPrimaryLayout) LayerName LayerWidget))
  (return _returnvalue))

(fn UnRegisterLayer
  (params (LayerName :type Gameplay%20Tag%20Structure))
  (bind _returnvalue (Default|UnRegisterLayer (CallFunction|GetPrimaryLayout) LayerName))
  (return _returnvalue))

(fn PushContenttoLayer
  (params (LayerName :type Gameplay%20Tag%20Structure) (WidgetClass :type User%20Widget%20Soft%20Class%20Reference))
  (bind _widget (Default|PushContenttoLayer (CallFunction|GetPrimaryLayout) LayerName WidgetClass))
  (return _widget))

(fn PopContentfromLayer
  (params (LayerName :type Gameplay%20Tag%20Structure))
  (Default|PopContentfromLayer (CallFunction|GetPrimaryLayout) LayerName)
  (return))

(fn ClearAllLayers
  (Default|ClearAllLayers (CallFunction|GetPrimaryLayout)))

(fn ClearAllLayersExcept
  (params (ExceptionLayerName :type Gameplay%20Tag%20Structure))
  (Default|ClearAllLayersExept (CallFunction|GetPrimaryLayout) ExceptionLayerName))

(fn ClearLayer
  (params (LayerName :type Gameplay%20Tag%20Structure))
  (Default|ClearLayer (CallFunction|GetPrimaryLayout) LayerName)
  (return))